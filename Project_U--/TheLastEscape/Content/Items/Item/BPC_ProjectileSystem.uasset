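; Projectile component that moves its owning actor like a bullet along its initial forward vector, destroying it when a lifetime expires.
; Each tick it line-traces on Visibility to the next position, destroying the owner on a hit without applying damage, otherwise moving it and updating velocity.
; Mass-scaled gravity and quadratic drag alter only vertical velocity, with drag computed from the constant launch speed.
; Traces draw debug lines.
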(event EventBeginPlay
  (bind _returnvalue (Components|GetOwner))
  (Variables|Default|SetActorToIgnore _returnvalue)
  (Variables|Default|SetBulletVelocity (* (Transformation|GetActorForwardVector _returnvalue) (Variables|Default|GetBulletSpeed)))
  (Variables|Default|SetStartLocation (Transformation|GetActorLocation _returnvalue))
  (Variables|Default|SetIsBulletInitiated true)
  (Utilities|FlowControl|Delay (Variables|Default|GetBulletLifeTime))
  (Actor|DestroyActor (Components|GetOwner)))

(event EventTick
  (params (DeltaSeconds :type Float%20%28single-precision%29))
  (if (Variables|Default|GetIsBulletInitiated)
    (Variables|Default|SetDelta%20Time DeltaSeconds)
    (Variables|Default|SetStartLocation (Transformation|GetActorLocation (Components|GetOwner)))
    (Variables|Default|SetNextLocation (+ (Variables|Default|GetStartLocation) (* (Variables|Default|GetBulletVelocity) (Variables|Default|GetDelta%20Time))))
    (bind (_outhit _returnvalue) (Collision|LineTraceByChannel (Variables|Default|GetStartLocation) (Variables|Default|GetNextLocation) "TraceTypeQuery1" false (Utilities|Array|MakeArray (Variables|Default|GetActorToIgnore)) "ForDuration" true "(R=1.000000,G=0.000000,B=0.000000,A=1.000000)" "(R=0.000000,G=1.000000,B=0.000000,A=1.000000)" 1e+01))
    (if _returnvalue
      (Actor|DestroyActor (Components|GetOwner))
      (else
        (Transformation|SetActorLocation (Components|GetOwner) (Variables|Default|GetNextLocation) false false)
        (Variables|Default|SetBulletVelocity (CallFunction|CalculateGravandDeceleration (Variables|Default|GetBulletVelocity)))))))

(fn CalculateGravandDeceleration
  (params (Velocity :type Vector))
  (return (+ Velocity (* (Math|Vector|MakeVector 0.0 0.0 (+ (CallFunction|DragForce (Variables|Default|GetAirDensity) (Variables|Default|GetBulletSpeed) (Variables|Default|GetCrossSection) (Variables|Default|GetDragCoefficiency)) (* (* (Variables|Default|GetGravity) 1e+02 2e+02) (Variables|Default|GetBulletMass) -1.0))) (Variables|Default|GetDelta%20Time)))))

(fn DragForce
  (params (AirDensity :type Float%20%28double-precision%29) (BulletSpeed :type Float%20%28double-precision%29) (CrossSection :type Float%20%28double-precision%29) (DragCoefficiency :type Float%20%28double-precision%29))
  (return (* (/ (* (* (* AirDensity (Math|Float|Square BulletSpeed)) CrossSection) DragCoefficiency) 2.0) -1.0)))