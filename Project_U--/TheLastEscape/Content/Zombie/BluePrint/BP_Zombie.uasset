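; Zombie enemy that chases the player via PawnSensing and AIMoveTo, flags attacks at close range, and works with an AIC_Zombie controller.
; Timer-delayed attacks sphere-trace along the right arm to deal random damage.
; BPCHp handles hit and per-tick Molotov burn damage; death disables capsule collision, then destroys the actor after a delay.
; Flash stun temporarily zeroes sight radius while Tick passes the player's location to the controller.
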(event OnSeePawn(PawnSensing)
  (params (Pawn :type Pawn%20Object%20Reference))
  (bind _asbp_player (Utilities|Casting|CastToBP_Player Pawn))
  (AI|AIMoveTo self "0, 0, 0" _asbp_player 5.0 false
    (:then
      (if (< (Math|Vector|Distance2D(Vector) (Transformation|GetActorLocation (Game|GetPlayerCharacter 0)) (Transformation|GetActorLocation self)) 2e+02)
        (Variables|Default|SetIsAttack true)
        (else
          (Variables|Default|SetIsAttack false))))))

(event Custom|Start%20Attack
  (bind _returnvalue (Utilities|Time|SetTimerbyEvent (delegate Custom|Attack) 0.1))
  (Variables|Default|SetAttack%20Timer%20Handler _returnvalue))

(event Custom|Attack
  (bind (_outhit _returnvalue) (Collision|SphereTraceByChannel (Transformation|GetWorldLocation (Variables|Default|GetRightArm)) (Transformation|GetWorldLocation (Variables|Default|GetRightHand)) 1e+01 "TraceTypeQuery1" false 0 "ForDuration" true "(R=1.000000,G=0.000000,B=0.000000,A=1.000000)" "(R=0.000000,G=1.000000,B=0.000000,A=1.000000)" 1e+01))
  (if _returnvalue
    (if (Actor|ActorHasTag (.HitActor (Collision|BreakHitResult _outhit)) "Player")
      (Game|Damage|ApplyDamage (.HitActor (Collision|BreakHitResult _outhit)) (Math|Random|RandomFloatinRange 1e+01 2e+01) 0 self))))

(event Custom|Stop%20Attack
  (Utilities|Time|ClearandInvalidateTimerbyHandle (Variables|Default|GetAttack%20Timer%20Handler)))

(event EventBeginPlay
  (bind _asaic_zombie (Utilities|Casting|CastToAIC_Zombie (AI|GetAIController self)))
  (Default|SetTarget _asaic_zombie (Game|GetPlayerCharacter 0)))

(event Game|Damage|EventAnyDamage
  (params (Damage :type Float%20%28single-precision%29) (DamageType :type Damage%20Type%20Object%20Reference) (InstigatedBy :type Controller%20Object%20Reference) (DamageCauser :type Actor%20Object%20Reference))
  (Variables|Default|SetIsHit true)
  (Variables|Default|SetDamage%20Causer DamageCauser)
  (bind _isdead (Default|DecreaseHealth (Variables|Default|GetBPC_Hp) Damage))
  (bind _output_get (Variables|Default|SetIsDead _isdead))
  (if _output_get
    (Collision|SetCollisionEnabled (Variables|Collision|GetCapsuleComponent) "NoCollision")
    (Variables|Default|SetIsHit false)
    (Utilities|FlowControl|Delay 5.0)
    (Actor|DestroyActor)
    (else
      (Utilities|FlowControl|Delay 1.5)
      (Variables|Default|SetIsHit false))))

(event EventTick
  (params (DeltaSeconds :type Float%20%28single-precision%29))
  (Utilities|FlowControl|Sequence
    (:then_0
      (if (Variables|Default|GetIsFlashStunned)
        (bind _asaic_zombie (Utilities|Casting|CastToAIC_Zombie (AI|GetAIController self)))
        (Variables|Default|SetAs%20AIC%20Zombie _asaic_zombie)
        (Default|CheckLocation _asaic_zombie (Transformation|GetActorLocation (Game|GetPlayerCharacter 0)))))
    (:then_1
      ;[1 1 1] 화염병 피해
      (bind _confirmdead (Default|DecreaseHealthbyBurn (Variables|Default|GetBPC_Hp)))
      (bind _output_get (Variables|Default|SetIsDead _confirmdead))
      (if _output_get
        (Collision|SetCollisionEnabled (Variables|Collision|GetCapsuleComponent) "NoCollision")
        (Utilities|FlowControl|Delay 5.0)
        (Actor|DestroyActor)))
    (:then_2
      (CallFunction|EventFlash))))

(fn ConstructionScript)

(fn IsSight
  (bind _output_get (Variables|Default|Set주변%20시야각 (Variables|/Script/AIModule.PawnSensingComponent|GetPeripheralVisionAngle (Variables|Default|GetPawnSensing))))
  (return (< (.x (Transformation|GetActorLocation (Game|GetPlayerCharacter 0))) _output_get)))

(fn ResetListen
  (AI|Components|Blackboard|SetValueasBool (Variables|/Script/AIModule.AIController|GetBlackboard (AI|GetAIController self)) (Variables|Default|GetKey_IsListen) false))

(fn EventFlash
  (if (Variables|Default|GetIsFlashStunned)
    (if (>= (Variables|Default|GetFlashStunTime) 4.0)
      (Variables|Default|SetFlashStunTime 0.0)
      (Variables|/Script/AIModule.PawnSensingComponent|SetSightRadius (Variables|Default|GetPawnSensing) 5e+03)
      (Variables|Default|SetIsFlashStunned false)
      (Variables|Default|SetIsHit false)
      (else
        (Variables|Default|SetFlashStunTime (+ (Variables|Default|GetFlashStunTime) (Utilities|Time|GetWorldDeltaSeconds)))
        (Variables|/Script/AIModule.PawnSensingComponent|SetSightRadius (Variables|Default|GetPawnSensing) 0.0)))
    (else
      (return))))