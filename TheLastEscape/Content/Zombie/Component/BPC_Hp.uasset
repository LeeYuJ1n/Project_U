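; BPC_Hp is a health component for the zombie game that tracks current and maximum HP along with a death flag.
; It fills HP to maximum on BeginPlay, clamps healing at the maximum and damage at zero, and sets IsDead when HP runs out.
; A separate burn function drains HP at a fixed rate scaled by delta seconds while IsBurn is set; the component's Tick does nothing.
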(event EventBeginPlay
  (CallFunction|InitializeStat))

(event EventTick
  (params (DeltaSeconds :type Float%20%28single-precision%29)))

(fn IncreaseHealth
  (params (HpPoint :type Float%20%28double-precision%29))
  (Variables|Default|SetCurHp (+ (Variables|Default|GetCurHp) HpPoint))
  (if (> (Variables|Default|GetCurHp) (Variables|Default|GetMaxHp))
    (Variables|Default|SetCurHp (Variables|Default|GetMaxHp))))

(fn DecreaseHealth
  (params (Damage :type Float%20%28double-precision%29))
  (Variables|Default|SetCurHp (- (Variables|Default|GetCurHp) Damage))
  (if (<= (Variables|Default|GetCurHp) 0.0)
    (Variables|Default|SetCurHp 0.0)
    (bind _output_get (Variables|Default|SetIsDead true))
    (return _output_get)
    (else
      (Variables|Default|SetIsDead false))))

(fn InitializeStat
  (Variables|Default|SetCurHp (Variables|Default|GetMaxHp)))

(fn DecreaseHealthbyBurn
  (if (Variables|Default|GetIsBurn)
    (Variables|Default|SetCurHp (- (Variables|Default|GetCurHp) (* (Utilities|Time|GetWorldDeltaSeconds) 12.0)))
    (if (<= (Variables|Default|GetCurHp) 0.0)
      (Variables|Default|SetCurHp 0.0)
      (bind _output_get (Variables|Default|SetIsDead true))
      (return _output_get))))