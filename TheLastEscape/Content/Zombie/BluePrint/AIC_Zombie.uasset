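; AI controller for zombies that starts the BB_Zombie blackboard and BT_Zombie behavior tree on BeginPlay.
; Custom events write perception results into the blackboard: target player, location to check, and sighted and heard flags.
; CheckTargetVector stores the first player character's current position in the location key.
; Sensing logic lives outside this controller, which only relays values to the tree.
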(event Custom|Set%20Target
  (params (Target :type Object%20Object%20Reference))
  (AI|Components|Blackboard|SetValueasObject (Variables|Default|GetBlackboard) (Variables|Default|GetKey_Player) Target))

(event Custom|Check%20Location
  (params (TargetLocation :type Vector))
  (AI|Components|Blackboard|SetValueasVector (Variables|Default|GetBlackboard) (Variables|Default|GetKey_Location) TargetLocation))

(event Custom|Is%20Sighted
  (params (Is%20SIght :type Boolean))
  (AI|Components|Blackboard|SetValueasBool (Variables|Default|GetBlackboard) (Variables|Default|GetKey_IsSight) Is%20SIght))

(event Custom|Is%20Listen
  (params (BoolValue :type Boolean))
  (AI|Components|Blackboard|SetValueasBool (Variables|Default|GetBlackboard) (Variables|Default|GetKey_IsListen) BoolValue))

(event EventBeginPlay
  (Class|AIController|UseBlackboard "/Game/Zombie/AI/BB_Zombie.BB_Zombie")
  (AI|RunBehaviorTree "/Game/Zombie/AI/BT_Zombie.BT_Zombie"))

(fn ConstructionScript)

(fn CheckTargetVector
  (AI|Components|Blackboard|SetValueasVector (Variables|Default|GetBlackboard) (Variables|Default|GetKey_Location) (Transformation|GetActorLocation (Game|GetPlayerCharacter 0)))
  (return))