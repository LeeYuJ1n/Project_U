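; Zombie enemy Blueprint that senses by sight and hearing and relays what it detects to its AIC_Zombie controller.
; On BeginPlay it sets the player as the controller's target and clears the sight flag.
; PawnSensing events reset, then immediately set, the IsSight and IsListen Blackboard flags.
; Tick sends the player's location to the controller and, after a short Delay, passes both flags to it.
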(event OnSeePawn(PawnSensing)
  (params (Pawn :type Pawn%20Object%20Reference))
  (Utilities|FlowControl|Sequence
    (:then_0
      (CallFunction|ResetSight))
    (:then_1
      (AI|Components|Blackboard|SetValueasBool (Variables|/Script/AIModule.AIController|GetBlackboard (AI|GetAIController self)) (Variables|Default|GetIsSight) true))))

(event OnHearNoise(PawnSensing)
  (params (Instigator :type Pawn%20Object%20Reference) (Location :type Vector%20%28by%20ref%29 :default "0, 0, 0") (Volume :type Float%20%28single-precision%29))
  (Utilities|FlowControl|Sequence
    (:then_0
      (CallFunction|ResetListen))
    (:then_1
      (AI|Components|Blackboard|SetValueasBool (Variables|Default|GetBlackboard) (Variables|Default|GetIsListen) true))))

(event EventBeginPlay
  (bind _asaic_zombie (Utilities|Casting|CastToAIC_Zombie (AI|GetAIController self)))
  (Default|SetTarget _asaic_zombie (Game|GetPlayerCharacter 0))
  (CallFunction|ResetSight))

(event Collision|EventActorBeginOverlap
  (params (OtherActor :type Actor%20Object%20Reference)))

(event EventTick
  (params (DeltaSeconds :type Float%20%28single-precision%29))
  (bind _asaic_zombie (Utilities|Casting|CastToAIC_Zombie (AI|GetAIController self)))
  (Default|CheckLocation _asaic_zombie (Transformation|GetActorLocation (Game|GetPlayerCharacter 0)))
  (Utilities|FlowControl|Delay 0.2)
  (Default|IsSighted _asaic_zombie (ScalableFloat|GetValueasBool (Variables|Default|GetBlackboard) (Variables|Default|GetIsSight)))
  (Default|IsListen _asaic_zombie (ScalableFloat|GetValueasBool (Variables|Default|GetBlackboard) (Variables|Default|GetIsListen))))

(fn ConstructionScript)

(fn ResetSight
  (AI|Components|Blackboard|SetValueasBool (Variables|/Script/AIModule.AIController|GetBlackboard (AI|GetAIController self)) (Variables|Default|GetIsSight) false))

(fn ResetListen
  (AI|Components|Blackboard|SetValueasBool (Variables|/Script/AIModule.AIController|GetBlackboard (AI|GetAIController self)) (Variables|Default|GetIsListen) false))