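; Player combat component that performs melee hit detection for BP_Player and applies damage to the actor hit.
; StartAttackTrace schedules one non-looping AttackTrace after a brief delay, and StopAttackTrace clears that timer.
; AttackTrace switches on weapon status: a sphere trace for unarmed, capsule traces for Secondary and Prime, with rising damage.
; Helper functions derive trace endpoints from the right fist's transform, reaching further for each weapon tier.
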(event Custom|StartAttackTrace
  (bind _returnvalue (Utilities|Time|SetTimerbyEvent (delegate Custom|AttackTrace) 0.01))
  (Variables|Default|SetAttackTime _returnvalue))

(event Custom|AttackTrace
  (bind _player (Variables|Default|GetPlayer))
  (bind _player_2 (Variables|Default|GetPlayer))
  (bind _player_3 (Variables|Default|GetPlayer))
  (bind _rightfist (Variables|/Game/Character/BP_Player.BP_Player_C|GetRightFist _player_3))
  (bind _rightfist_2 (Variables|/Game/Character/BP_Player.BP_Player_C|GetRightFist _player))
  (bind _rightfist_3 (Variables|/Game/Character/BP_Player.BP_Player_C|GetRightFist _player_2))
  (bind (_start _end) (CallFunction|GetSecondaryLocation _rightfist))
  (bind (_start_2 _end_2) (CallFunction|GetPrimeLocation _rightfist_2))
  (bind (_start_3 _end_3) (CallFunction|GetHandLocation _rightfist_3))
  (switch Utilities|FlowControl|Switch|SwitchonEN_PlayerWeaponStatus (Variables|/Game/Character/BP_Player.BP_Player_C|GetCurrentWeaponStatus (Variables|Default|GetPlayer))
    (:NewEnumerator8
      (bind (_outhit _returnvalue) (Collision|SphereTraceByChannel _start_3 _end_3 1e+01 "TraceTypeQuery1" false 0 "None" true "(R=1.000000,G=0.000000,B=0.000000,A=1.000000)" "(R=0.000000,G=1.000000,B=0.000000,A=1.000000)" 7.0))
      (if _returnvalue
        (Game|Damage|ApplyDamage (.HitActor (Collision|BreakHitResult _outhit)) 3e+01 0 (Variables|Default|GetPlayer))))
    (:NewEnumerator2
      (bind (_outhit_2 _returnvalue_2) (Collision|CapsuleTraceByChannel _start _end 15.0 2e+01 "TraceTypeQuery1" false 0 "None" true "(R=1.000000,G=0.000000,B=0.000000,A=1.000000)" "(R=0.000000,G=1.000000,B=0.000000,A=1.000000)" 7.0))
      (if _returnvalue_2
        (Game|Damage|ApplyDamage (.HitActor (Collision|BreakHitResult _outhit_2)) 6e+01 0 (Variables|Default|GetPlayer))))
    (:NewEnumerator9
      (bind (_outhit_3 _returnvalue_3) (Collision|CapsuleTraceByChannel _start_2 _end_2 15.0 2e+01 "TraceTypeQuery1" false 0 "None" true "(R=1.000000,G=0.000000,B=0.000000,A=1.000000)" "(R=0.000000,G=1.000000,B=0.000000,A=1.000000)" 7.0))
      (if _returnvalue_3
        (Game|Damage|ApplyDamage (.HitActor (Collision|BreakHitResult _outhit_3)) 7e+01 0 (Variables|Default|GetPlayer))))))

(event Custom|StopAttackTrace
  (Utilities|Time|ClearandInvalidateTimerbyHandle (Variables|Default|GetAttackTime)))

(event EventBeginPlay
  (bind _asbp_player (Utilities|Casting|CastToBP_Player (Components|GetOwner)))
  (Utilities|IsValid _asbp_player
    (:Is%20Valid
      (bind _output_get (Variables|Default|SetPlayer _asbp_player))
      (Variables|Default|Set메시 (Variables|/Script/Engine.Character|GetMesh _output_get)))))

(event EventTick
  (params (DeltaSeconds :type Float%20%28single-precision%29)))

(fn GetHandLocation
  (params (Hand :type Scene%20Component%20Object%20Reference))
  (return (Transformation|GetWorldLocation Hand) (Math|Transform|TransformLocation (Transformation|GetWorldTransform Hand) (+ (Variables|/Script/Engine.SceneComponent|GetRelativeLocation Hand) (Math|Vector|MakeVector 2e+01 0.0 0.0)))))

(fn GetSecondaryLocation
  (params (Hand :type Scene%20Component%20Object%20Reference))
  (return (Transformation|GetWorldLocation Hand) (Math|Transform|TransformLocation (Transformation|GetWorldTransform Hand) (+ (Variables|/Script/Engine.SceneComponent|GetRelativeLocation Hand) (Math|Vector|MakeVector 4e+01 0.0 0.0)))))

(fn GetPrimeLocation
  (params (Hand :type Scene%20Component%20Object%20Reference))
  (return (Transformation|GetWorldLocation Hand) (Math|Transform|TransformLocation (Transformation|GetWorldTransform Hand) (+ (Variables|/Script/Engine.SceneComponent|GetRelativeLocation Hand) (Math|Vector|MakeVector 5e+01 0.0 0.0)))))