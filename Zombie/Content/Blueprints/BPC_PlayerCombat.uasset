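; Actor component that handles melee attack tracing for the owning BP_Player, caching the player and its mesh on BeginPlay.
; StartAttackTrace sets a short, non-looping timer that runs one debug-drawn sphere trace on the Visibility channel at the right fist.
; GetHandLocation builds the trace segment from the fist component's world transform and an offset, while StopAttackTrace clears the timer.
; The trace's hit result is not yet used.
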(event Custom|StartAttackTrace
  (bind _returnvalue (Utilities|Time|SetTimerbyEvent (delegate Custom|AttackTrace) 0.01))
  (Variables|Default|SetAttackTime _returnvalue))

(event Custom|AttackTrace
  (bind _player (Variables|Default|GetPlayer))
  (bind _rightfist (Variables|/Game/Character/BP_Player.BP_Player_C|GetRightFist _player))
  (bind (_start _end) (CallFunction|GetHandLocation _rightfist))
  (Collision|SphereTraceByChannel _start _end 1e+01 "TraceTypeQuery1" false 0 "ForDuration" true "(R=1.000000,G=0.000000,B=0.000000,A=1.000000)" "(R=0.000000,G=1.000000,B=0.000000,A=1.000000)" 7.0))

(event Custom|StopAttackTrace
  (Utilities|Time|ClearandInvalidateTimerbyHandle (Variables|Default|GetAttackTime)))

(event EventBeginPlay
  (bind _asbp_player (Utilities|Casting|CastToBP_Player (Components|GetOwner)))
  (Utilities|IsValid _asbp_player
    (:Is%20Valid
      (bind _output_get (Variables|Default|SetPlayer _asbp_player))
      (Variables|Default|Set메시 (Variables|/Script/Engine.Character|GetMesh _output_get)))))

(event EventTick
  (params (DeltaSeconds :type Float%20%28single-precision%29)))

(fn GetHandLocation
  (params (Hand :type Scene%20Component%20Object%20Reference))
  (return (Transformation|GetWorldLocation Hand) (Math|Transform|TransformLocation (Transformation|GetWorldTransform Hand) (+ (Variables|/Script/Engine.SceneComponent|GetRelativeLocation Hand) (Math|Vector|MakeVector 2e+01 0.0 0.0)))))