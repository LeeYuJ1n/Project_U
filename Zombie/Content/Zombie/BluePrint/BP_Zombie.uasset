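; Zombie enemy pawn that senses and attacks the player, takes damage and is destroyed shortly after death.
; PawnSensing sets sight and hearing Blackboard flags, while Tick passes player location and, after a delay, those flags to AIC_Zombie.
; Attacks use a one-shot timer to sphere-trace along the right arm, applying random damage to Player-tagged actors.
; Incoming damage goes through BPCHp, setting hit or death state and disabling capsule collision on death.
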(event OnSeePawn(PawnSensing)
  (params (Pawn :type Pawn%20Object%20Reference))
  (while (ScalableFloat|GetValueasBool (Variables|Default|GetBlackboard) (Variables|Default|GetIsSight))
    (CallFunction|ResetSight))
  (AI|Components|Blackboard|SetValueasBool (Variables|/Script/AIModule.AIController|GetBlackboard (AI|GetAIController self)) (Variables|Default|GetIsSight) true))

(event OnHearNoise(PawnSensing)
  (params (Instigator :type Pawn%20Object%20Reference) (Location :type Vector%20%28by%20ref%29 :default "0, 0, 0") (Volume :type Float%20%28single-precision%29))
  (Utilities|FlowControl|Sequence
    (:then_0
      (CallFunction|ResetListen))
    (:then_1
      (AI|Components|Blackboard|SetValueasBool (Variables|Default|GetBlackboard) (Variables|Default|GetIsListen) true))))

(event Custom|Start%20Attack
  (bind _returnvalue (Utilities|Time|SetTimerbyEvent (delegate Custom|Attack) 0.01))
  (Variables|Default|SetAttack%20Timer%20Handler _returnvalue))

(event Custom|Attack
  (bind (_outhit _returnvalue) (Collision|SphereTraceByChannel (Transformation|GetWorldLocation (Variables|Default|GetRightArm)) (Transformation|GetWorldLocation (Variables|Default|GetRightHand)) 1e+01 "TraceTypeQuery1" false 0 "ForDuration" true "(R=1.000000,G=0.000000,B=0.000000,A=1.000000)" "(R=0.000000,G=1.000000,B=0.000000,A=1.000000)" 1e+01))
  (if _returnvalue
    (if (Actor|ActorHasTag (.HitActor (Collision|BreakHitResult _outhit)) "Player")
      (Game|Damage|ApplyDamage (.HitActor (Collision|BreakHitResult _outhit)) (Math|Random|RandomFloatinRange 1e+01 2e+01) 0 self))))

(event Custom|Stop%20Attack
  (Utilities|Time|ClearandInvalidateTimerbyHandle (Variables|Default|GetAttack%20Timer%20Handler)))

(event EventBeginPlay
  (bind _asaic_zombie (Utilities|Casting|CastToAIC_Zombie (AI|GetAIController self)))
  (Default|SetTarget _asaic_zombie (Game|GetPlayerCharacter 0)))

(event Collision|EventActorBeginOverlap
  (params (OtherActor :type Actor%20Object%20Reference)))

(event EventTick
  (params (DeltaSeconds :type Float%20%28single-precision%29))
  (bind _asaic_zombie (Utilities|Casting|CastToAIC_Zombie (AI|GetAIController self)))
  (Default|CheckLocation _asaic_zombie (Transformation|GetActorLocation (Game|GetPlayerCharacter 0)))
  (Utilities|FlowControl|Delay 0.2)
  (Default|IsSighted _asaic_zombie (ScalableFloat|GetValueasBool (Variables|Default|GetBlackboard) (Variables|Default|GetIsSight)))
  (Default|IsListen _asaic_zombie (ScalableFloat|GetValueasBool (Variables|Default|GetBlackboard) (Variables|Default|GetIsListen))))

(event Game|Damage|EventAnyDamage
  (params (Damage :type Float%20%28single-precision%29) (DamageType :type Damage%20Type%20Object%20Reference) (InstigatedBy :type Controller%20Object%20Reference) (DamageCauser :type Actor%20Object%20Reference))
  (Variables|Default|SetDamage%20Causer DamageCauser)
  (Variables|Default|SetIsHit true)
  (bind _isdead (Default|DecreaseHealth (Variables|Default|GetBPC_Hp) Damage))
  (bind _output_get (Variables|Default|SetIsDead _isdead))
  (if _output_get
    (Collision|SetCollisionEnabled (Variables|Collision|GetCapsuleComponent) "NoCollision")
    (Utilities|FlowControl|Delay 5.0)
    (Actor|DestroyActor)
    (else
      (Utilities|FlowControl|Delay 0.5)
      (Variables|Default|SetIsHit false))))

(fn ConstructionScript)

(fn ResetSight
  (AI|Components|Blackboard|SetValueasBool (Variables|/Script/AIModule.AIController|GetBlackboard (AI|GetAIController self)) (Variables|Default|GetIsSight) false))

(fn ResetListen
  (AI|Components|Blackboard|SetValueasBool (Variables|/Script/AIModule.AIController|GetBlackboard (AI|GetAIController self)) (Variables|Default|GetIsListen) false))