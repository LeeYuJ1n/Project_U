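; AI controller for zombies that runs the BT_Zombie behavior tree on the BB_Zombie blackboard.
; Setter events write target, location, sight, hearing, hit and death state to the blackboard.
; Perception updates for Player-tagged actors set sight and hearing true, plus target and 2D distance, without checking sense type or stimulus success.
; Updates from other actors clear both flags.
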(event OnTargetPerceptionUpdated(AIPerception)
  (params (Actor :type Actor%20Object%20Reference) (Stimulus :type AI%20Stimulus%20Structure))
  (bind _blackboard (Variables|Default|GetBlackboard))
  (if (Actor|ActorHasTag Actor "Player")
    (AI|Components|Blackboard|SetValueasBool _blackboard (Variables|Default|GetKey_IsSight) true)
    (AI|Components|Blackboard|SetValueasObject _blackboard (Variables|Default|GetKey_Player) Actor)
    (AI|Components|Blackboard|SetValueasBool _blackboard (Variables|Default|GetKey_IsListen) true)
    (AI|Components|Blackboard|SetValueasFloat _blackboard (Variables|Default|GetKey_Distance) (CallFunction|GetTargetDistance Actor))
    (else
      (AI|Components|Blackboard|SetValueasBool (Variables|Default|GetBlackboard) (Variables|Default|GetKey_IsSight) false)
      (AI|Components|Blackboard|SetValueasBool (Variables|Default|GetBlackboard) (Variables|Default|GetKey_IsListen) false))))

(event Custom|Set%20Target
  (params (Target :type Object%20Object%20Reference))
  (AI|Components|Blackboard|SetValueasObject (Variables|Default|GetBlackboard) (Variables|Default|GetKey_Player) Target))

(event Custom|IsHit
  (params (IsHit :type Boolean))
  (AI|Components|Blackboard|SetValueasBool (Variables|Default|GetBlackboard) (Variables|Default|GetKey_IsHit) IsHit))

(event Custom|Check%20Location
  (params (TargetLocation :type Vector))
  (AI|Components|Blackboard|SetValueasVector (Variables|Default|GetBlackboard) (Variables|Default|GetKey_Location) TargetLocation))

(event Custom|IsDead
  (params (IsDead :type Boolean))
  (AI|Components|Blackboard|SetValueasBool (Variables|Default|GetBlackboard) (Variables|Default|GetKey_IsDead) IsDead))

(event Custom|Is%20Sighted
  (params (Is%20SIght :type Boolean))
  (AI|Components|Blackboard|SetValueasBool (Variables|Default|GetBlackboard) (Variables|Default|GetKey_IsSight) Is%20SIght))

(event Custom|Is%20Listen
  (params (IsListen :type Boolean))
  (AI|Components|Blackboard|SetValueasBool (Variables|Default|GetBlackboard) (Variables|Default|GetKey_IsListen) IsListen))

(event EventBeginPlay
  (Class|AIController|UseBlackboard "/Game/Zombie/AI/BB_Zombie.BB_Zombie")
  (AI|RunBehaviorTree "/Game/Zombie/AI/BT_Zombie.BT_Zombie"))

(fn ConstructionScript)

(fn GetTargetDistance
  (params (Actor :type Actor%20Object%20Reference))
  (return (Math|Vector|Distance2D(Vector) (Transformation|GetActorLocation Actor) (Transformation|GetActorLocation))))